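; Snowball actor that explodes with smoke, sound and area damage, either after a short delay or on hitting a Timmy.
; Each path sphere-overlaps for Timmy actors and damages only the first, if its game has started.
; The timed path destroys the snowball on authority or when nothing overlaps; the hit path's destroy sits behind contradictory authority switches.
; Sound and destruction use MC events; leftover movement-freeze logic is disconnected.
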(event `self.ReceiveBeginPlay`
  (`KismetSystemLibrary.Delay` 1.4)
  (`/Engine/EditorBlueprintResources/StandardMacros.IsValid` self
    (:`Is Valid`
      (`NiagaraFunctionLibrary.SpawnSystemAtLocation` "/Game/Assets/Niagara/NS_Impact_Smoke.NS_Impact_Smoke" (`self.K2_GetActorLocation`))
      (`self.MC_PlaySnowballExplosionSound`)
      (bind (_outactors _returnvalue) (`KismetSystemLibrary.SphereOverlapActors` (`self.K2_GetActorLocation`) 500.0 (`|MakeArray` "ObjectTypeQuery1" "ObjectTypeQuery2" "ObjectTypeQuery3" "ObjectTypeQuery11" :!type "EObjectTypeQuery Enum") "/Game/Common/Characters/Timmy.Timmy_C" (`|MakeArray` self :!type "Actor Object Reference")))
      (if _returnvalue
        (bind _astimmy (cast `/Game/Common/Characters/Timmy` (`|GetArrayItem` _outactors)))
        (if (`/Game/Common/Characters/Timmy.HasGameStarted?` _astimmy)
          (`GameplayStatics.ApplyDamage` _astimmy (`self.Damage`) null self)
          (`/Engine/EditorBlueprintResources/ActorMacros.Switch Has Authority`
            (:`Authority`
              (`self.MC_DestroySnowball`)
              (`self.K2_DestroyActor`))))
        (else
          (`self.K2_DestroyActor`))))))

(event `self.ReceiveHit`
  (params (MyComp :type "PrimitiveComponent Object Reference") (Other :type "Actor Object Reference") (OtherComp :type "PrimitiveComponent Object Reference") (bSelfMoved :type Boolean) (HitLocation :type "Vector Structure") (HitNormal :type "Vector Structure") (NormalImpulse :type "Vector Structure") (Hit :type "HitResult Structure (by ref)"))
  (cast `/Game/Common/Characters/Timmy` Other)
  (`NiagaraFunctionLibrary.SpawnSystemAtLocation` "/Game/Assets/Niagara/NS_Impact_Smoke.NS_Impact_Smoke" (`self.K2_GetActorLocation`))
  (`self.MC_PlaySnowballExplosionSound`)
  (bind (_outactors _returnvalue) (`KismetSystemLibrary.SphereOverlapActors` (`self.K2_GetActorLocation`) 500.0 (`|MakeArray` "ObjectTypeQuery1" "ObjectTypeQuery2" "ObjectTypeQuery3" :!type "EObjectTypeQuery Enum") "/Game/Common/Characters/Timmy.Timmy_C" (`|MakeArray` self :!type "Actor Object Reference")))
  (if _returnvalue
    (bind _astimmy (cast `/Game/Common/Characters/Timmy` (`|GetArrayItem` _outactors)))
    (if (`/Game/Common/Characters/Timmy.HasGameStarted?` _astimmy)
      (`GameplayStatics.ApplyDamage` _astimmy (`self.Damage`) null self)
      (`/Engine/EditorBlueprintResources/ActorMacros.Switch Has Authority`
        (:`Authority`
          (`/Engine/EditorBlueprintResources/ActorMacros.Switch Has Authority`
            (:`Remote`
              (`self.MC_DestroySnowball`)
              (`self.K2_DestroyActor`))))))))

(event `MC_PlaySnowballExplosionSound`
  (`GameplayStatics.PlaySoundAtLocation` "/Game/Sound/HandWhip/SFX_HandWhipActivate_Cue.SFX_HandWhipActivate_Cue" (`self.K2_GetActorLocation`) (struct) 1.0 1.0 0.0 null null null null))

(event `MC_DestroySnowball`
  (`self.K2_DestroyActor`))

(fn `UserConstructionScript`)