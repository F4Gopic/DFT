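; BP_VentInteraction is an interactable vent that shows an interaction prompt and passes vent use to the interacting actor.
; On BeginPlay it labels its WB_InteractionFeedback widget component as "Vent".
; SetFocused shows the widget and uses a short retriggerable delay to hide it once focus calls stop arriving.
; Interact calls HandleVentMessage on the interacting actor, leaving the vent behavior to that actor.
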(event `self.ReceiveBeginPlay`
  (`self.Setup_InteractionWidget`))

(event `/Game/Blueprints/Interfaces/BPI_InteractHelper.Set Focused`
  (`SceneComponent.SetVisibility` (`self.Widget`) true false)
  (`KismetSystemLibrary.RetriggerableDelay` 0.1)
  (`SceneComponent.SetVisibility` (`self.Widget`) false false))

(event `/Game/Common/Characters/BPI/BPI_Interact.Interact`
  (params (InteractingActor :type "Actor Object Reference"))
  (message `/Game/Common/Characters/BPI/BPI_Tools.Handle_Vent` InteractingActor))

(fn `Setup_InteractionWidget`
  (bind _aswb_interaction_feedback (cast `/Game/Common/UI/WB_InteractionFeedback` (`WidgetComponent.GetWidget` (`self.Widget`))))
  (`/Game/Common/UI/WB_InteractionFeedback.UpdateWidget` _aswb_interaction_feedback "Vent"))

(fn `UserConstructionScript`)