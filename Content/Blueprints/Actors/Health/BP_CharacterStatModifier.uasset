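; Health pickup actor that adjusts a character's health by a configurable amount when the primary action is pressed.
; SetupActor stores the target character, and the primary action event calls a consume event, whose SR prefix suggests a server RPC.
; That event sends the amount to the character through AdjustHealthMessage, with no removal of the pack afterwards.
; The construction script applies the mesh from a variable.
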(event `/Game/Common/Characters/BPI/BPI_Tools.Setup_Actor`
  (params (Character :type "/Game/Common/Characters/MainCharacter Object Reference"))
  (set `self.CID_Character` Character))

(event `/Game/Common/Characters/BPI/BPI_Inputs.Input_PrimaryActionPressed`
  (`self.SR_ConsumeHealthPack`))

(event `SR_ConsumeHealthPack`
  (message `/Game/Common/Characters/BPI/BPI_CharacterStats.Adjust_Health` (`self.CID_Character`) (`self.AmountOfHealthModified`)))

(fn `UserConstructionScript`
  (`StaticMeshComponent.SetStaticMesh` (`self.Mesh`) (`self.SMMesh`)))