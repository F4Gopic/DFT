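; Throwable turret actor that auto-targets and shoots Timmy pawns within its sensing radius.
; Server Tick drives MC-prefixed events that pick the nearest visible target via sphere overlap, rotate the top at constant speed with clamped pitch, and fire.
; Each tick with line of sight, a forward trace triggers impact FX and sound on any hit, damaging only the target.
; FindBestTarget, UpdateTurretRotation and UpdateFire functions duplicate those events but are uncalled here.
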(event `self.ReceiveTick`
  (params (DeltaSeconds :type "Float (single-precision)"))
  (`/Engine/EditorBlueprintResources/ActorMacros.Switch Has Authority`
    (:`Authority`
      (`self.MC_FindBestTarget`)
      (`self.Target`
        (:`then`
          (`/Engine/EditorBlueprintResources/ActorMacros.Switch Has Authority`
            (:`Authority`
              (`self.MC_UpdateTurretRotation` DeltaSeconds)
              (`/Engine/EditorBlueprintResources/ActorMacros.Switch Has Authority`
                (:`Authority`
                  (`self.MC_UpdateFire`))))))
        (:`else`)))))

(event `MC_FXAndSound`
  (params (`Impact Affect Location` :type "Vector Structure") (`Sound Play Location` :type "Vector Structure"))
  (`NiagaraFunctionLibrary.SpawnSystemAtLocation` "/Game/Assets/Niagara/NS_Impact.NS_Impact" `Impact Affect Location`)
  (`NiagaraFunctionLibrary.SpawnSystemAtLocation` "/Niagara/DefaultAssets/Templates/Systems/SimpleExplosion.SimpleExplosion" (`SceneComponent.K2_GetComponentLocation` (`self.ShotExplosionLocation`)) (struct) (0.1 0.1 0.1))
  (`GameplayStatics.PlaySoundAtLocation` "/Game/Sound/Pistol/SFX_GunShoot.SFX_GunShoot" `Sound Play Location` (struct) 1.0 1.0 0.0 null null null null))

(event `MC_UpdateFire`
  (bind _target (`self.Target`))
  (bind _returnvalue (`SceneComponent.K2_GetComponentLocation` (`self.SM_TurretTop`)))
  (bind _target_2 (`self.Target`)
    (:`then`
      (bind _return_value (`/Game/Blueprints/FunctionLibraries/BFL_GenericFunctions.Has Line Of Sight` (`SceneComponent.K2_GetComponentLocation` (`self.SM_TurretTop`)) (`self.K2_GetActorLocation` _target_2) (`|MakeArray` self (`self.Target`) :!type "Actor Object Reference")))
      (if _return_value
        (bind (_outhit _returnvalue_2) (`KismetSystemLibrary.LineTraceSingle` :`Start` _returnvalue :`End` (+ _returnvalue (* (`KismetMathLibrary.GetForwardVector` (`SceneComponent.K2_GetComponentRotation` (`self.SM_TurretTop`))) 5000.0)) :`TraceChannel` "TraceTypeQuery1" :`DrawDebugType` "ForDuration"))
        (if _returnvalue_2
          (bind (_bblockinghit _binitialoverlap _time _distance _location _impactpoint _normal _impactnormal _physmat _hitactor) (`GameplayStatics.BreakHitResult` _outhit))
          (`self.MC_FXAndSound` _location (`self.K2_GetActorLocation`))
          (if (== _hitactor _target)
            (`GameplayStatics.ApplyDamage` _target 1.0 null self)))))
    (:`else`)))

(event `MC_UpdateTurretRotation`
  (params (DeltaSeconds :type "Float (double-precision)"))
  (bind _output_get (set `self.NewTurretTopRotation` (`KismetMathLibrary.RInterpTo_Constant` (`SceneComponent.K2_GetComponentRotation` (`self.SM_TurretTop`)) (`KismetMathLibrary.FindLookAtRotation` (`SceneComponent.K2_GetComponentLocation` (`self.SM_TurretTop`)) (`self.K2_GetActorLocation` (`self.Target`))) DeltaSeconds (`self.RotationSpeed`))))
  (`SceneComponent.K2_SetWorldRotation` (`self.SM_TurretTop`) (`KismetMathLibrary.MakeRotator` (.roll _output_get) (`KismetMathLibrary.ClampAngle` (.pitch _output_get) -45.0 75.0) (.yaw _output_get)) false false))

(event `MC_FindBestTarget`
  (set `self.BestDistance` (+ (`self.SensingRadius`) 1.0))
  (bind _outactors (`KismetSystemLibrary.SphereOverlapActors` (`self.K2_GetActorLocation`) (`self.SensingRadius`) (`|MakeArray` "ObjectTypeQuery3" :!type "EObjectTypeQuery Enum") "/Game/Common/Characters/Timmy.Timmy_C"))
  (for _array_element _outactors
    (bind _output_get (set `self.CurrentTarget` _array_element))
    (bind _output_get_2 (set `self.CurrentDistance` (`self.GetDistanceTo` _output_get self)))
    (if (or (< _output_get_2 (`self.BestDistance`)) (not (`KismetSystemLibrary.IsValid` (`self.BestTarget`))))
      (bind _return_value (`/Game/Blueprints/FunctionLibraries/BFL_GenericFunctions.Has Line Of Sight` (`SceneComponent.K2_GetComponentLocation` (`self.SM_TurretTop`)) (`self.K2_GetActorLocation` (`self.CurrentTarget`)) (`|MakeArray` self (`self.CurrentTarget`) :!type "Actor Object Reference")))
      (if _return_value
        (set `self.BestTarget` (`self.CurrentTarget`))
        (set `self.BestDistance` (`self.CurrentDistance`)))))
  (set `self.Target` (`self.BestTarget`)))

(fn `FindBestTarget`
  (set `self.BestDistance` (+ (`self.SensingRadius`) 1.0))
  (bind _outactors (`KismetSystemLibrary.SphereOverlapActors` (`self.K2_GetActorLocation`) (`self.SensingRadius`) (`|MakeArray` "ObjectTypeQuery3" :!type "EObjectTypeQuery Enum") "/Game/Common/Characters/Timmy.Timmy_C"))
  (for _array_element _outactors
    (bind _output_get (set `self.CurrentTarget` _array_element))
    (bind _output_get_2 (set `self.CurrentDistance` (`self.GetDistanceTo` _output_get self)))
    (if (or (< _output_get_2 (`self.BestDistance`)) (not (`KismetSystemLibrary.IsValid` (`self.BestTarget`))))
      (bind _return_value (`/Game/Blueprints/FunctionLibraries/BFL_GenericFunctions.Has Line Of Sight` (`SceneComponent.K2_GetComponentLocation` (`self.SM_TurretTop`)) (`self.K2_GetActorLocation` (`self.CurrentTarget`)) (`|MakeArray` self (`self.CurrentTarget`) :!type "Actor Object Reference")))
      (if _return_value
        (set `self.BestTarget` (`self.CurrentTarget`))
        (set `self.BestDistance` (`self.CurrentDistance`)))))
  (set `self.Target` (`self.BestTarget`)))

(fn `UpdateFire`
  (bind _target (`self.Target`))
  (bind _returnvalue (`SceneComponent.K2_GetComponentLocation` (`self.SM_TurretTop`)))
  (bind _target_2 (`self.Target`)
    (:`then`
      (bind _return_value (`/Game/Blueprints/FunctionLibraries/BFL_GenericFunctions.Has Line Of Sight` (`SceneComponent.K2_GetComponentLocation` (`self.SM_TurretTop`)) (`self.K2_GetActorLocation` _target_2) (`|MakeArray` self (`self.Target`) :!type "Actor Object Reference")))
      (if _return_value
        (bind (_outhit _returnvalue_2) (`KismetSystemLibrary.LineTraceSingle` :`Start` _returnvalue :`End` (+ _returnvalue (* (`KismetMathLibrary.GetForwardVector` (`SceneComponent.K2_GetComponentRotation` (`self.SM_TurretTop`))) 5000.0)) :`TraceChannel` "TraceTypeQuery1" :`DrawDebugType` "ForDuration"))
        (if _returnvalue_2
          (bind (_bblockinghit _binitialoverlap _time _distance _location _impactpoint _normal _impactnormal _physmat _hitactor) (`GameplayStatics.BreakHitResult` _outhit))
          (`self.MC_FXAndSound` _location (`self.K2_GetActorLocation`))
          (if (== _hitactor _target)
            (`GameplayStatics.ApplyDamage` _target 1.0 null self)))))
    (:`else`)))

(fn `UpdateTurretRotation`
  (params (DeltaSeconds :type "Float (double-precision)"))
  (locals (NewRotation :type "Rotator Structure" :default (struct)))
  (bind _output_get (set `local.NewRotation` (`KismetMathLibrary.RInterpTo_Constant` (`SceneComponent.K2_GetComponentRotation` (`self.SM_TurretTop`)) (`KismetMathLibrary.FindLookAtRotation` (`SceneComponent.K2_GetComponentLocation` (`self.SM_TurretTop`)) (`self.K2_GetActorLocation` (`self.Target`))) (`local.DeltaSeconds`) (`self.RotationSpeed`))))
  (`SceneComponent.K2_SetWorldRotation` (`self.SM_TurretTop`) (`KismetMathLibrary.MakeRotator` (.roll _output_get) (`KismetMathLibrary.ClampAngle` (.pitch _output_get) -45.0 75.0) (.yaw _output_get)) false false))

(fn `UserConstructionScript`)