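; BP_ItemBox is an interactable loot box that scatters random pickups when first opened.
; Interact sets the RepNotify Opened flag, which swaps the box material, then spawns loot and calls the open-sound event that stops the idle audio.
; Three BP_PickupItems spawn inside SpawnVolume, each chosen by re-rolling random DT_PickupItems rows against SpawnPercentage.
; SetFocused briefly shows the prompt widget and custom-depth highlight, using a retriggerable delay to clear them.
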(event `self.ReceiveBeginPlay`
  (`ActorComponent.Activate` (`self.ItemBoxSoundFX`) true)
  (`self.Setup_InteractionWidget`))

(event `/Game/Common/Characters/BPI/BPI_Interact.Interact`
  (params (InteractingActor :type "Actor Object Reference"))
  (if (not (`self.Opened?`))
    (set `self.Opened?` true)
    (`self.SpawnItems`)
    (`self.MC_OpenChestSoundFX`)))

(event `/Game/Common/Characters/BPI/BPI_Interact.SetFocused`
  (`SceneComponent.SetVisibility` (`self.Widget`) true false)
  (`PrimitiveComponent.SetRenderCustomDepth` (`self.Mesh`) true)
  (`KismetSystemLibrary.RetriggerableDelay` 0.1)
  (`PrimitiveComponent.SetRenderCustomDepth` (`self.Mesh`) false)
  (`SceneComponent.SetVisibility` (`self.Widget`) false false))

(event `MC_OpenChestSoundFX`
  (`GameplayStatics.PlaySoundAtLocation` "/Engine/EditorSounds/GamePreview/StartPlayInEditor_Cue.StartPlayInEditor_Cue" (`self.K2_GetActorLocation`) (struct) 1.0 1.0 0.0 null null null null)
  (`AudioComponent.Stop` (`self.ItemBoxSoundFX`)))

(event `OpenItemBox`
  (`PrimitiveComponent.SetMaterial` (`self.Mesh`) 0 "/Game/Common/Props/Box/Materials/MI_Box_Body.MI_Box_Body"))

(event `SpawnItems`
  (bind _output_get (set `self.LootSpawnAmount` 3))
  (bind _counter (`/Engine/EditorBlueprintResources/StandardMacros.Do N` _output_get :!label _label)
    (:`Exit`
      (`self.SpawnActualItem`)
      (if (not (== _counter (`self.LootSpawnAmount`)))
        (goto _label)))))

(event `SpawnActualItem`
  (bind _outrownames (`DataTableFunctionLibrary.GetDataTableRowNames` "/Game/Blueprints/Data/DT_PickupItems.DT_PickupItems" :!label _label_2))
  (bind _returnvalue (`|GetDataTableRow` "/Game/Blueprints/Data/DT_PickupItems.DT_PickupItems" (`KismetArrayLibrary.Array_Random` _outrownames))
    (:`then`
      (bind (_id _name _sm_item _spawnpercentage) (break `/Game/Blueprints/Data/S_PickupItem` _returnvalue))
      (if (<= (`KismetMathLibrary.RandomFloatInRange` 0.0 100.0) _spawnpercentage)
        (`|SpawnActorFromClass` "/Game/Common/Items/BP_PickupItem.BP_PickupItem_C" (`KismetMathLibrary.MakeTransform` (`KismetMathLibrary.RandomPointInBoundingBox` (`SceneComponent.K2_GetComponentLocation` (`self.SpawnVolume`)) (`BoxComponent.GetUnscaledBoxExtent` (`self.SpawnVolume`)))) "AdjustIfPossibleButAlwaysSpawn" "MultiplyWithRoot" null _id null)
        (else
          (goto _label_2))))))

(fn `OnRep_Opened?`
  (`self.OpenItemBox`))

(fn `Setup_InteractionWidget`
  (bind _aswb_interaction_feedback (cast `/Game/Common/UI/WB_InteractionFeedback` (`WidgetComponent.GetWidget` (`self.Widget`))))
  (`/Game/Common/UI/WB_InteractionFeedback.UpdateWidget` _aswb_interaction_feedback "Item Box"))

(fn `UserConstructionScript`)

(fn `Vent`
  (returns (VentAttachLocation :type "Vector Structure"))
  (return (0.0 0.0 0.0)))