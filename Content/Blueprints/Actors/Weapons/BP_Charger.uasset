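; Charger weapon Blueprint that builds up shot damage while the primary action is held and fires a line-trace shot on release.
; If it has ammo and is not reloading, pressing starts a looping timer that raises Damage to a cap.
; Release clears the timer, spends ammo, fires and resets Damage.
; MC-prefixed events drive charge audio, switching to a ready cue after a delay, while Tick prints Damage for debugging.
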(event `self.ReceiveTick`
  (params (DeltaSeconds :type "Float (single-precision)"))
  (`KismetSystemLibrary.PrintString` (`KismetStringLibrary.Conv_DoubleToString` (`self.Damage`))))

(event `self.SR_PrimaryAction`
  (params (`Pressed?` :type Boolean))
  (bind _rateoffire (`self.RateOfFire`))
  (if `Pressed?`
    (`self.CanShootCharger?`
      (:`true`
        (`self.MC_ChargerSequenceBackground`)
        (`self.MC_ChargerSequence`)
        (set `self.IsChargingUp` true)
        (bind _returnvalue (`KismetSystemLibrary.K2_SetTimerDelegate` (delegate `ShootingCharger`) _rateoffire true (* _rateoffire -1.0)))
        (set `self.TH_Shooting` _returnvalue)))
    (else
      (`KismetSystemLibrary.K2_ClearAndInvalidateTimerHandle` (`self.TH_Shooting`))
      (set `self.IsChargingUp` false)
      (`self.CanShootCharger?`
        (:`true`
          (`/Engine/EditorBlueprintResources/StandardMacros.DecrementInt` (`self.Ammo`)
            (:`  `
              (`self.MC_Shoot`)
              (`self.LineTrace_Shot`)
              (set `self.Damage` 50.0)
              (`self.MC_StopChargerSequence`)
              (`self.MC_ResetChargeSequence`))))))))

(event `ShootingCharger`
  (if (<= (`self.Damage`) 399.0)
    (set `self.Damage` (+ (`self.Damage`) 50.0))))

(event `MC_ChargerSequenceBackground`
  (`AudioComponent.Play` (`self.ChargerChargeUpBackground`) 0.0))

(event `MC_ChargerSequence`
  (bind _chargerchargesequence (`self.ChargerChargeSequence`))
  (bind _chargerchargesequence_2 (`self.ChargerChargeSequence`))
  (`AudioComponent.SetSound` _chargerchargesequence_2 "/Game/Sound/Charger/SFX_ChargerChargeUpSteady_Cue.SFX_ChargerChargeUpSteady_Cue")
  (`AudioComponent.Play` _chargerchargesequence_2 0.0)
  (`KismetSystemLibrary.Delay` 7.0)
  (if (`self.IsChargingUp`)
    (`AudioComponent.SetSound` _chargerchargesequence "/Game/Sound/Charger/SFX_ChargerChargeUpReady_Cue.SFX_ChargerChargeUpReady_Cue")
    (`AudioComponent.Play` _chargerchargesequence 0.0)))

(event `MC_StopChargerSequence`
  (`AudioComponent.Stop` (`self.ChargerChargeUpBackground`))
  (`AudioComponent.Stop` (`self.ChargerChargeSequence`)))

(event `MC_ResetChargeSequence`
  (`AudioComponent.SetSound` (`self.ChargerChargeSequence`) "/Game/Sound/Charger/SFX_ChargerChargeUpSteady_Cue.SFX_ChargerChargeUpSteady_Cue"))

(fn `UserConstructionScript`
  (`parent.UserConstructionScript`))