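; BP_CoreWeapon is a networked gun actor with automatic fire, ammo and timed reload, linked to its owning character by SetupActor.
; Server events run a looping fire timer and the reload delay, while multicasts play sounds and impact effects.
; Each shot line-traces from the character's camera, offset by spring arm length, unless that character is Timmy.
; Hits apply damage and notify the character when the target implements BPI_TimmyDamageCounter.
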(event `/Game/Common/Characters/BPI/BPI_Tools.Setup_Actor`
  (params (Character :type "/Game/Common/Characters/Character/MainCharacter Object Reference"))
  (bind _output_get (set `self.CID_Character` Character))
  (add `/Game/Common/Characters/Character/MainCharacter.SendDamageDealt` _output_get (delegate `SendDamageDealt`)))

(event `SendDamageDealt`
  (set `/Game/Common/Characters/Character/MainCharacter.DamageDealtOnShot` (`self.Damage`) (`self.CID_Character`)))

(event `/Game/Common/Characters/BPI/BPI_Inputs.Input_PrimaryActionPressed`
  ;[1 1 1] Inputs
  (`self.SR_PrimaryAction` true))

(event `/Game/Common/Characters/BPI/BPI_Inputs.Input_PrimaryActionReleased`
  ;[1 1 1] Inputs
  (`self.SR_PrimaryAction` false))

(event `SR_PrimaryAction`
  (params (`Pressed?` :type Boolean))
  (bind _rateoffire (`self.RateOfFire`))
  ;[1 1 1] Shooting
  (if `Pressed?`
    (bind _returnvalue (`KismetSystemLibrary.K2_SetTimerDelegate` (delegate `Shooting`) _rateoffire true (* _rateoffire -1.0)))
    (set `self.TH_Shooting` _returnvalue)
    (else
      (`KismetSystemLibrary.K2_ClearAndInvalidateTimerHandle` (`self.TH_Shooting`)))))

(event `Shooting`
  ;[1 1 1] Shooting
  (`self.CanShoot?`
    (:`true`
      (`/Engine/EditorBlueprintResources/StandardMacros.DecrementInt` (`self.Ammo`)
        (:`  `
          (`self.MC_Shoot`)
          (`self.LineTrace_Shot`))))))

(event `MC_Shoot`
  ;[1 1 1] Shooting
  (`GameplayStatics.SpawnSoundAttached` (`self.ShootSoundFX`) (`self.Mesh`) "None" (0.0 0.0 0.0) (struct) "KeepRelativeOffset" false 1.0 1.0 0.0 null null))

(event `MC_SpawnImpact`
  (params (Location :type "Vector Structure") (Normal :type "Vector Structure"))
  ;[1 1 1] Shooting
  (`NiagaraFunctionLibrary.SpawnSystemAtLocation` (`self.ImpactFX`) Location (`KismetMathLibrary.Conv_VectorToRotator` Normal)))

(event `/Game/Common/Characters/BPI/BPI_Inputs.Input_Reload`
  ;[1 1 1] Reload
  (`self.SR_Reload`))

(event `SR_Reload`
  ;[1 1 1] Reload
  (`self.CanReload?`
    (:`true`
      (set `self.Reloading?` true)
      (`self.MC_Reload`)
      (`KismetSystemLibrary.Delay` (`self.ReloadDuration`))
      (set `self.Ammo` (`self.MaxAmmo`))
      (set `self.Reloading?` false))))

(event `MC_Reload`
  ;[1 1 1] Reload
  (`GameplayStatics.SpawnSoundAttached` (`self.ReloadSoundFX`) (`self.Mesh`) "None" (0.0 0.0 0.0) (struct) "KeepRelativeOffset" false 1.0 1.0 0.0 null null))

(fn `LineTrace_Shot`
  (bind _cid_character (`self.CID_Character`))
  (bind _camera (`/Game/Common/Characters/Character/MainCharacter.Camera` _cid_character))
  (bind _returnvalue (`SceneComponent.K2_GetComponentLocation` _camera))
  (bind _returnvalue_2 (`SceneComponent.GetForwardVector` _camera))
  (if (not (`/Game/Common/Characters/Character/MainCharacter.IsTimmy?` _cid_character))
    (bind (_outhit _returnvalue_3) (`KismetSystemLibrary.LineTraceSingle` (+ _returnvalue (* _returnvalue_2 (`SpringArmComponent.TargetArmLength` (`/Game/Common/Characters/Character/MainCharacter.SpringArm` _cid_character)))) (+ _returnvalue (* _returnvalue_2 (`self.ShootingRange`))) "TraceTypeQuery1" false (`|MakeArray` (`self.CID_Character`) :!type "Actor Object Reference")))
    (if _returnvalue_3
      (bind (_bblockinghit _binitialoverlap _time _distance _location _impactpoint _normal _impactnormal _physmat _hitactor) (`GameplayStatics.BreakHitResult` _outhit))
      (`self.MC_SpawnImpact` _location _normal)
      (bind _returnvalue_4 (`GameplayStatics.ApplyDamage` _hitactor (`self.Damage`) null self))
      (if (`KismetSystemLibrary.DoesImplementInterface` _hitactor "/Game/Common/Characters/BPI/BPI_TimmyDamageCounter.BPI_TimmyDamageCounter_C")
        (set `self.DamageDealtOnWeaponShot` _returnvalue_4)
        (`/Game/Common/Characters/Character/MainCharacter.ReceiveDamageDealtToTimmy` (`self.CID_Character`) _hitactor)))))

(fn `UserConstructionScript`
  (`StaticMeshComponent.SetStaticMesh` (`self.Mesh`) (`self.Weapon_Mesh`)))