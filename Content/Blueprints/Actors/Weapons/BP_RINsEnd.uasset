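; BP_RINsEnd is a hitscan weapon Blueprint for the RINsEnd gun, built on a parent weapon class.
; Primary press calls SRPrimaryAction, which checks ammo and reload state, decrements ammo, then calls MCShoot and LineTraceShot.
; A DoOnce with no visible reset lets the first shot trigger a delayed camera shake, multicast through the character.
; The reload input is empty, and the construction script's material assignments are disconnected.
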(event `/Game/Common/Characters/BPI/BPI_Inputs.Input_PrimaryActionPressed`
  (`self.SR_PrimaryAction` true))

(event `/Game/Common/Characters/BPI/BPI_Inputs.Input_PrimaryActionReleased`
  (`self.SR_PrimaryAction` false))

(event `self.SR_PrimaryAction`
  (params (`Pressed?` :type Boolean))
  (if `Pressed?`
    (`self.CanShoot?`
      (:`true`
        (`/Engine/EditorBlueprintResources/StandardMacros.DecrementInt` (`self.Ammo`)
          (:`  `
            (`self.MC_Shoot`)
            (`self.LineTrace_Shot`)
            (`/Engine/EditorBlueprintResources/StandardMacros.DoOnce` false
              (:`Completed`
                (`KismetSystemLibrary.Delay` 5.0)
                (`self.SR_StartCameraShake`)))))))))

(event `/Game/Common/Characters/BPI/BPI_Inputs.Input_Reload`)

(event `SR_StartCameraShake`
  (`/Game/Common/Characters/MainCharacter.MULTICAST_PlayRINsEndCameraShake` (`self.CID_Character`)))

(event `GoingToJobMIJK4g?3KfyR`)

(fn `UserConstructionScript`
  (`parent.UserConstructionScript`))