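; Timmy turret tool that places a BP_ThrowableTurret on the surface in front of the character holding it.
; On primary press, a capsule trace sized to the character runs forward, then a second sweeps down from its end to find the ground.
; On a hit, only the Remote authority branch calls the SR events that spawn the turret at the impact point and remove the tool from the character.
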(event `/Game/Common/Characters/BPI/BPI_Inputs.Input_PrimaryActionPressed`
  (`self.SR_PrimaryActionOV` true))

(event `/Game/Common/Characters/BPI/BPI_Inputs.Input_PrimaryActionReleased`
  (`self.SR_PrimaryActionOV` false))

(event `SR_PrimaryActionOV`
  (params (Pressed :type Boolean))
  (if Pressed
    (bind _cid_character (`self.CID_Character`)
      (:`then`
        (bind _returnvalue (`self.K2_GetActorLocation` _cid_character))
        (bind _capsulecomponent (`Character.CapsuleComponent` _cid_character))
        (bind _returnvalue_2 (`CapsuleComponent.GetUnscaledCapsuleRadius` _capsulecomponent))
        (bind _returnvalue_3 (`CapsuleComponent.GetUnscaledCapsuleHalfHeight` _capsulecomponent))
        (bind _outhit (`KismetSystemLibrary.CapsuleTraceSingle` _returnvalue (+ _returnvalue (* (`KismetMathLibrary.GetForwardVector` (`self.K2_GetActorRotation` _cid_character)) 212.0)) _returnvalue_2 _returnvalue_3 "TraceTypeQuery1"))
        (bind (_bblockinghit _binitialoverlap _time _distance _location _impactpoint _normal _impactnormal _physmat _hitactor _hitcomponent _hitbonename _bonename _hititem _elementindex _faceindex _tracestart _traceend) (`GameplayStatics.BreakHitResult` _outhit))
        (bind (_outhit_2 _returnvalue_4) (`KismetSystemLibrary.CapsuleTraceSingle` _traceend (`KismetMathLibrary.MakeVector` (.x _traceend) (.y _traceend) (- (.z _traceend) 1000.0)) _returnvalue_2 _returnvalue_3 "TraceTypeQuery1"))
        (if _returnvalue_4
          (`/Engine/EditorBlueprintResources/ActorMacros.Switch Has Authority`
            (:`Remote`
              (`self.SR_SpawnThrowableTurret` (`.ImpactPoint` (`GameplayStatics.BreakHitResult` _outhit_2)))
              (`/Engine/EditorBlueprintResources/ActorMacros.Switch Has Authority`
                (:`Remote`
                  (`self.SR_RemoveTimmyTurret`)))))))
      (:`else`))))

(event `SR_RemoveTimmyTurret`
  (`/Game/Common/Characters/MainCharacter.RemoveTool` (`self.CID_Character`)))

(event `SR_SpawnThrowableTurret`
  (params (Location :type "Vector Structure"))
  (`|SpawnActorFromClass` "/Game/Blueprints/Actors/ThrowableItems/Turret/BP_ThrowableTurret.BP_ThrowableTurret_C" (`KismetMathLibrary.MakeTransform` Location) "AdjustIfPossibleButAlwaysSpawn" "MultiplyWithRoot" self null))

(fn `UserConstructionScript`
  (`parent.UserConstructionScript`))