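; BP_SnowballLauncher is a weapon that fires physics-driven snowballs repeatedly while the primary action is held.
; Pressing starts a looping RateOfFire timer, offset by a negative start delay to fire without waiting, and releasing clears it.
; Each shot decrements Ammo without checking it, calls MCShoot, then spawns BP_Snowball at the Arrow and launches it forward and slightly upward by impulse.
; Tick prints a debug "Hello".
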(event `self.ReceiveTick`
  (params (DeltaSeconds :type "Float (single-precision)"))
  (`KismetSystemLibrary.PrintString` "Hello"))

(event `self.SR_PrimaryAction`
  (params (`Pressed?` :type Boolean))
  (bind _rateoffire (`self.RateOfFire`))
  (if `Pressed?`
    (bind _returnvalue (`KismetSystemLibrary.K2_SetTimerDelegate` (delegate `ShootingOV`) _rateoffire true (* _rateoffire -1.0)))
    (set `self.TH_Shooting` _returnvalue)
    (else
      (`KismetSystemLibrary.K2_ClearAndInvalidateTimerHandle` (`self.TH_Shooting`)))))

(event `ShootingOV`
  (`/Engine/EditorBlueprintResources/StandardMacros.DecrementInt` (`self.Ammo`)
    (:`  `
      (`self.MC_Shoot`)
      (`self.ShootSnowballProjectile`))))

(fn `ShootSnowballProjectile`
  (bind (_returnvalue_x _returnvalue_y) (`KismetMathLibrary.BreakVector` (* (`KismetMathLibrary.GetForwardVector` (`self.K2_GetActorRotation`)) 1000.0)))
  (bind _returnvalue (`|SpawnActorFromClass` "/Game/Assets/Snowball/BP_Snowball.BP_Snowball_C" (`KismetMathLibrary.MakeTransform` (`SceneComponent.K2_GetComponentLocation` (`self.Arrow`))) "AdjustIfPossibleButAlwaysSpawn" "MultiplyWithRoot" null null))
  (`/Engine/EditorBlueprintResources/StandardMacros.IsValid` _returnvalue
    (:`Is Valid`
      (`PrimitiveComponent.AddImpulse` (`/Game/Assets/Snowball/BP_Snowball.Mesh` _returnvalue) (`KismetMathLibrary.MakeVector` _returnvalue_x _returnvalue_y 100.0) "None" false))))

(fn `UserConstructionScript`
  (`parent.UserConstructionScript`))