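; BP_GenericNote is an interactable note actor that holds text for the main character to read.
; On BeginPlay it writes its name into a WB_InteractionFeedback widget, which SetFocused shows briefly, using a retriggerable delay to hide it once focus calls stop.
; Interact passes the note to MainCharacter's InteractWithNote on authority only.
; SendGenericNoteData returns the note text, while Vent just returns a zero vector.
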(event `self.ReceiveBeginPlay`
  (bind _aswb_interaction_feedback (cast `/Game/Common/UI/WB_InteractionFeedback` (`WidgetComponent.GetWidget` (`self.Widget`))))
  (`/Game/Common/UI/WB_InteractionFeedback.UpdateWidget` _aswb_interaction_feedback (`KismetTextLibrary.Conv_StringToText` (`self.Name`))))

(event `/Game/Common/Characters/BPI/BPI_Interact.Interact`
  (params (InteractingActor :type "Actor Object Reference"))
  (bind _asmain_character (cast `/Game/Common/Characters/MainCharacter` InteractingActor))
  (`/Engine/EditorBlueprintResources/ActorMacros.Switch Has Authority`
    (:`Authority`
      (`/Game/Common/Characters/MainCharacter.InteractWithNote` _asmain_character self))))

(event `/Game/Common/Characters/BPI/BPI_Interact.SetFocused`
  (`SceneComponent.SetVisibility` (`self.Widget`) true false)
  (`KismetSystemLibrary.RetriggerableDelay` 0.1)
  (`SceneComponent.SetVisibility` (`self.Widget`) false false))

(fn `SendGenericNoteData`
  (returns (OutText :type Text))
  (return (`self.NoteText`)))

(fn `UserConstructionScript`)

(fn `Vent`
  (returns (VentAttachLocation :type "Vector Structure"))
  (return (0.0 0.0 0.0)))