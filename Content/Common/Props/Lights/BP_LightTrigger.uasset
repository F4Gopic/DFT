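; BP_LightTrigger is a trigger volume that notifies linked lights when main characters enter or leave its collision.
; It finds every BP_TriggerLight whose LightTriggerID matches IDToInteract and messages it on overlap begin and end.
; Overlap counts limit messages to the first character entering and the last one leaving.
; The first successful light trigger also starts the Timmy_BasementBoss battle through a DoOnce, with a leftover debug print.
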(event `self.Collision.OnComponentBeginOverlap`
  (params (OverlappedComponent :type "PrimitiveComponent Object Reference") (OtherActor :type "Actor Object Reference") (OtherComp :type "PrimitiveComponent Object Reference") (OtherBodyIndex :type Integer) (bFromSweep :type Boolean) (SweepResult :type "HitResult Structure (by ref)"))
  (cast `/Game/Common/Characters/MainCharacter` OtherActor)
  (bind _outactors (`GameplayStatics.GetAllActorsOfClass` "/Game/Common/Props/Lights/BP_TriggerLight.BP_TriggerLight_C"))
  (for _array_element _outactors
    (if (and (`KismetStringLibrary.EqualEqual_StrStr` (`/Game/Common/Props/Lights/BP_TriggerLight.LightTriggerID` _array_element) (`self.IDToInteract`)) (not (>= (`KismetArrayLibrary.Array_Length` (`PrimitiveComponent.GetOverlappingActors` (`self.Collision`) "/Game/Common/Characters/MainCharacter.MainCharacter_C")) 2)))
      (message `/Game/Common/Characters/BPI/BPI_LightTrigger.OverlapTrigger` _array_element (`self.IDToInteract`))
      (`/Engine/EditorBlueprintResources/StandardMacros.DoOnce` false
        (:`Completed`
          (bind _returnvalue (`GameplayStatics.GetActorOfClass` "/Game/Common/Characters/Timmy_BasementBoss.Timmy_BasementBoss_C"))
          (`/Game/Common/Characters/Timmy_BasementBoss.StartBossBattle` _returnvalue)
          (`KismetSystemLibrary.PrintString` "aaa"))))))

(event `self.Collision.OnComponentEndOverlap`
  (params (OverlappedComponent :type "PrimitiveComponent Object Reference") (OtherActor :type "Actor Object Reference") (OtherComp :type "PrimitiveComponent Object Reference") (OtherBodyIndex :type Integer))
  (cast `/Game/Common/Characters/MainCharacter` OtherActor)
  (bind _outactors (`GameplayStatics.GetAllActorsOfClass` "/Game/Common/Props/Lights/BP_TriggerLight.BP_TriggerLight_C"))
  (for _array_element _outactors
    (if (and (`KismetStringLibrary.EqualEqual_StrStr` (`/Game/Common/Props/Lights/BP_TriggerLight.LightTriggerID` _array_element) (`self.IDToInteract`)) (not (`KismetArrayLibrary.Array_IsValidIndex` (`PrimitiveComponent.GetOverlappingActors` (`self.Collision`) "/Game/Common/Characters/MainCharacter.MainCharacter_C"))))
      (message `/Game/Common/Characters/BPI/BPI_LightTrigger.EndOverlapTrigger` _array_element))))

(fn `UserConstructionScript`)